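; BP_EnemyBat is a sprite-based bat enemy that patrols horizontally along world X, starting in a random direction.
; Non-player capsule hits with an X normal reverse movement, with a DoOnce and short delay debouncing repeated turns.
; RotateBat mirrors the sprite by flipping its X scale to match the direction.
; On death it runs the parent EnemyDied logic, then destroys itself.
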(event OnComponentHit(CapsuleComponent)
  (params (HitComponent :type Primitive%20Component%20Object%20Reference) (OtherActor :type Actor%20Object%20Reference) (OtherComp :type Primitive%20Component%20Object%20Reference) (NormalImpulse :type Vector :default "0, 0, 0") (Hit :type Hit%20Result%20Structure%20%28by%20ref%29))
  (if (!= OtherActor (Game|Player|GetPlayerPawn 0))
    (if (!= (.X (Math|Vector|BreakVector (.normal Hit))) 0.0)
      (Utilities|FlowControl|DoOnce false
        (:Completed
          (Variables|Default|SetMoveRight (not (Variables|Default|GetMoveRight)))
          (CallFunction|RotateBat)
          (Utilities|FlowControl|Delay 0.1)
          (CallFunction|ResetDirectionChangeCheck))))))

(event Custom|ResetDirectionChangeCheck
  (Utilities|FlowControl|DoOnce false) ; enters at Reset
)

(event EventBeginPlay
  (Variables|Default|SetMoveRight (Math|Random|RandomBool))
  (CallFunction|RotateBat))

(event EventTick
  (params (DeltaSeconds :type Float%20%28single-precision%29))
  (Pawn|Input|AddMovementInput "1.000000, 0, 0" (select (Variables|Default|GetMoveRight) 1.0 -1.0) false))

(fn ConstructionScript
  (|CallParentFunction))

(fn EnemyDied
  (|CallParentFunction)
  (Actor|DestroyActor))

(fn RotateBat
  (bind _sprite (Variables|Default|GetSprite))
  (bind _returnvalue (Transformation|GetWorldScale _sprite))
  (Transformation|SetWorldScale3D (Variables|Default|GetSprite) (Math|Vector|MakeVector (* (Math|Float|Absolute(Float) (.x _returnvalue)) (select (Variables|Default|GetMoveRight) -1.0 1.0)) (.y _returnvalue) (.z _returnvalue))))